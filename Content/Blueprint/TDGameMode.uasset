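; Tower defense game mode that initializes a level from a level data input.
; SetupLevel switches the menu widget to the HUD if needed, with a leftover "Hello" debug print, then applies the data.
; Applying it pushes starting coin, life and mana to TDPlayerController, then loads two fixed unit commons and the base tower resources.
; The Health value is passed along but never used.
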(fn `ApplyLevelData`
  (params (LevelData :type "LevelData Object Reference"))
  (bind _astdplayer_controller (cast `TDPlayerController` (`GameplayStatics.GetPlayerController` 0)))
  (`TDPlayerController.UpdateValue` _astdplayer_controller (`LevelData.DefaultCoin` LevelData) "Coin")
  (`TDPlayerController.UpdateValue` _astdplayer_controller (`LevelData.DefaultLife` LevelData) "Life")
  (`TDPlayerController.UpdateValue` _astdplayer_controller (`LevelData.DefaultMana` LevelData) "Mana")
  (`self.LoadTDUnitCommons` (`|MakeArray` "/Game/Data/Unit/Light01Common.Light01Common" "/Game/Data/Unit/BarracksUnit01Com.BarracksUnit01Com" :!type "TDUnitCommonData Object Reference"))
  (`self.LoadTowerResources` "/Game/Data/Tower/BaseTowerData.BaseTowerData"))

(fn `SetupLevel`
  (params (`New Level Data` :type "LevelData Object Reference"))
  (if (not (== (`self.CurrentWidget`) "/Game/Blueprint/UI/HUD.HUD"))
    (`KismetSystemLibrary.PrintString` "Hello")
    (`self.ChangeMenuWidget` "/Game/Blueprint/UI/HUD.HUD_C"))
  (`self.ApplyLevelData` `New Level Data`))

(fn `UserConstructionScript`)