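; Player controller for the tower defense game that runs a top-down orthographic camera and touch panning.
; LevelChange spawns the camera if needed and sets its ortho width and pan limit from map size.
; Holding touch pans horizontally within that limit, keeping the visible HUD tower action menu on its tower.
; A touch while awaiting the next touch hides that menu; range-checked barracks rally-point placement exists but is disconnected.
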(event `LevelChange`
  (params (`Map Size` :type "Vector2D Structure"))
  ;[1 1 1] Set Initial Camera
  (`/Engine/EditorBlueprintResources/StandardMacros.IsValid` (`self.ViewCameraActor`)
    (:`Is Valid`
      _)
    (:`Is Not Valid`
      (bind _returnvalue (`|SpawnActorFromClass` "/Script/Engine.CameraActor" (`KismetMathLibrary.MakeTransform` (0.0 0.0 500.0) (struct :`Pitch` -90.0 :`Roll` -90.0)) "Undefined" "OverrideRootScale" null null))
      (bind _output_get (set `self.ViewCameraActor` _returnvalue))
      (`self.SetViewTargetWithBlend` _output_get)
      (bind _cameracomponent (`CameraActor.CameraComponent` _returnvalue))
      (`CameraComponent.SetProjectionMode` _cameracomponent "Orthographic")
      (`CameraComponent.SetConstraintAspectRatio` _cameracomponent false)))
  (`self.SetCameraFitToMap` `Map Size`))

(event `Testing_pc`)

(event `InputAction|PlayerTouched` :consume false
  (params (Key :type "Key Structure"))
  (:`Pressed`
    (if (`self.IsWaitingForNextTouch`)
      (set `self.IsWaitingForNextTouch` false)
      (`HUDWidget.HideTowerActionMenu` (`self.HUDWidget`))
      (else
        (`/Engine/EditorBlueprintResources/StandardMacros.IsValid` (`self.ViewCameraActor`)
          (:`Is Valid`
            (set `self.IsCameraPanning` true))))))
  (:`Released`
    (set `self.IsCameraPanning` false)))

(event `InputAxis|ScreenScrollX`
  (params (AxisValue :type "Float (single-precision)"))
  (bind _returnvalue (* AxisValue (`self.CameraSpeed`)))
  (bind _returnvalue_x (`KismetMathLibrary.BreakVector` (`SceneComponent.K2_GetComponentLocation` (`Actor.RootComponent` (`self.ViewCameraActor`)))))
  ;[1 1 1] 카메라 패닝
  (if (`self.IsCameraPanning`)
    (if (< (`KismetMathLibrary.Abs` (+ _returnvalue _returnvalue_x)) (`self.PanThreshold`))
      (`SceneComponent.K2_AddWorldOffset` (`Actor.RootComponent` (`self.ViewCameraActor`)) (`KismetMathLibrary.MakeVector` _returnvalue) false false)
      ;;[1 1 1] TowerActionMenu Position
      (bind _ashud (cast `/Game/Blueprint/UI/HUD` (`self.HUDWidget`)))
      (bind _toweractionmenu (`/Game/Blueprint/UI/HUD.TowerActionMenu` _ashud))
      (if (`|EnumEquality` (`Widget.GetVisibility` _toweractionmenu) "Visible")
        (`/Game/Blueprint/UI/TowerActionMenu.Set Postion to Tower Postion` _toweractionmenu)))))

(fn `SetCameraFitToMap`
  (params (`Map Size` :type "Vector2D Structure"))
  (bind (_x _y) (`KismetMathLibrary.BreakVector2D` `Map Size`))
  (bind _returnvalue (* (`CameraComponent.AspectRatio` (`CameraActor.CameraComponent` (`self.ViewCameraActor`))) _y))
  (set `self.PanThreshold` (/ (- _x _returnvalue) 2.0))
  (`CameraComponent.SetOrthoWidth` (`CameraActor.CameraComponent` (`self.ViewCameraActor`)) _returnvalue))

(fn `UserConstructionScript`)