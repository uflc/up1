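; LockOnDebuff is a flipbook-based debuff component that makes its TDCharacter owner take extra damage while locked on.
; DebuffStart disables looping and, once per activation, binds DamageAmplify to the owner's OnTakeDamage, which applies a truncated tenth of each hit as additional damage.
; DebuffEnd plays the lock-on end flipbook and sets a timer for its length, after which EffectEnd unbinds the amplifier and destroys the component.
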(event `self.DebuffStart`
  (if (not (`self.bIsDebuffActivated`))
    (`self.SetLooping` false)
    (set `self.bIsDebuffActivated` true)
    (bind _astdcharacter (cast `TDCharacter` (`self.GetOwner`)))
    (add `TDCharacter.OnTakeDamage` _astdcharacter (delegate `DamageAmplify`))))

(event `self.DebuffEnd`
  (`self.SetFlipbook` "/Game/Image/Tower/SkillEffect/LockOn/Lockon_End.Lockon_End")
  (`self.PlayFromStart`)
  (`KismetSystemLibrary.K2_SetTimerDelegate` (delegate `Effect End`) (`self.GetFlipbookLength`)))

(event `DamageAmplify`
  (params (InDamage :type "Damage Structure (by ref)"))
  (bind _astdcharacter (cast `TDCharacter` (`self.GetOwner`)))
  (`StatsComponent.TakeDamage` (`TDCharacter.Stats` _astdcharacter) (make `Damage` :`Damage` (`KismetMathLibrary.FTrunc` (* (`.Damage` (break `Damage` InDamage)) 0.1)))))

(event `Effect End`
  (set `self.bIsDebuffActivated` false)
  (bind _astdcharacter (cast `TDCharacter` (`self.GetOwner`)))
  (remove `TDCharacter.OnTakeDamage` _astdcharacter (delegate `DamageAmplify`))
  (`self.K2_DestroyComponent`))