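; Level actor that spawns waves of AI enemy units from per-level wave data.
; TestSpawn takes a wave index and passes each entry of that wave to a spawn subevent.
; The subevent waits for the entry's start time, then spawns its unit class with BT_Enemy at the indexed starting location.
; A custom ForLoopWithDelay macro repeats the spawn for the entry's amount, spaced by its delay.
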(event `self.TestSpawn`
  (params (WaveIdx :type Integer))
  (for _array_element (`.Wave` (break `WaveDataArray` (`|GetArrayItem` (`self.LevelWaveData`) WaveIdx)))
    (`self.Spawn_Subevent` _array_element)))

(event `Spawn_Subevent`
  (params (WaveData :type "WaveData Structure"))
  (bind (_locationidx _unitclass _startingtime _amount _delay) (break `WaveData` WaveData))
  (`KismetSystemLibrary.Delay` _startingtime)
  (`self.ForLoopWithDelay` 1 _amount _delay
    (:`LoopBody`
      (`AIBlueprintHelperLibrary.SpawnAIFromClass` _unitclass "/Game/Blueprint/AI/BT_Enemy.BT_Enemy" (`|GetArrayItem` (`self.EnemyStartingLocation`) _locationidx) (struct) true))))

(fn `UserConstructionScript`)