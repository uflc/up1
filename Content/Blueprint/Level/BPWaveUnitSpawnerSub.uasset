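; Sub-spawner that spawns one enemy group of a wave for its root BPWaveUnitSpawner, using its LevelWaveData.
; After a start delay, a looping timer spawns BT_Enemy AI at the root's first start location and writes its destination to the blackboard.
; Once the amount is reached, it waits, then decrements the root's active sub-spawner count.
; Only the last one triggers the next wave and destroys itself.
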(event `self.WaveSpawnSub`
  (bind _rootspawner (`self.RootSpawner`))
  (bind (_locationidx _unitclass _startingtime _amount _delay) (break `WaveData` (`self.LevelWaveData`)))
  (`KismetSystemLibrary.PrintString` "CustomEvent")
  (`/Engine/EditorBlueprintResources/StandardMacros.IsValid` _rootspawner
    (:`Is Valid`
      (cast `/Game/Blueprint/Level/BPWaveUnitSpawner` _rootspawner
        (:`then`
          (`KismetSystemLibrary.RetriggerableDelay` _startingtime)
          (bind _returnvalue (`KismetSystemLibrary.K2_SetTimerDelegate` (delegate `SpawnUnit`) _delay true)))
        (:`CastFailed`
          (`KismetSystemLibrary.PrintString` "not valid" :!label _label)
          (`self.K2_DestroyActor`))))
    (:`Is Not Valid`
      (goto _label))))

(event `SpawnUnit`
  (bind (_locationidx _unitclass _startingtime _amount) (break `WaveData` (`self.LevelWaveData`)))
  (bind _returnvalue (`AIBlueprintHelperLibrary.SpawnAIFromClass` _unitclass "/Game/Blueprint/AI/BT_Enemy.BT_Enemy" (`|GetArrayItem` (`WaveUnitSpawner.EnemyStartingLocation` (`self.RootSpawner`))) (struct) true))
  (`BlackboardComponent.SetValueAsVector` (`AIBlueprintHelperLibrary.GetBlackboard` _returnvalue) (`self.DestinationKey`) (`|GetArrayItem` (`WaveUnitSpawner.EnemyDestination` (`self.RootSpawner`)) _locationidx))
  (`KismetSystemLibrary.PrintString` "spawn unit")
  (bind _result (`/Engine/EditorBlueprintResources/StandardMacros.IncrementInt` (`self.Amountcounter`))
    (:`  `
      (if (>= _result _amount)
        (`KismetSystemLibrary.K2_ClearAndInvalidateTimerHandle` (stale `self.WaveSpawnSub` _returnvalue))
        (`KismetSystemLibrary.RetriggerableDelay` 10.0)
        (`self.ToNextWave`)))))

(fn `ToNextWave`
  (bind _rootspawner (`self.RootSpawner`))
  (bind _asbpwave_unit_spawner (cast `/Game/Blueprint/Level/BPWaveUnitSpawner` _rootspawner))
  (bind _result (`/Engine/EditorBlueprintResources/StandardMacros.DecrementInt` (`WaveUnitSpawner.ActiveSubSpawnerNumber` _rootspawner))
    (:`  `
      (if (<= _result 0)
        (bind _result_2 (`/Engine/EditorBlueprintResources/StandardMacros.IncrementInt` (`/Game/Blueprint/Level/BPWaveUnitSpawner.CurrentLevel` _asbpwave_unit_spawner))
          (:`  `
            (`/Game/Blueprint/Level/BPWaveUnitSpawner.Wave Nth Spawn` _asbpwave_unit_spawner _result_2)
            (`self.K2_DestroyActor`)))))))

(fn `UserConstructionScript`)