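; EnemyMelee05 is a melee enemy unit that splits into a follow-up enemy, EnemyMelee05_1, when it dies.
; On Die it saves the Destination vector from its AI blackboard before running the parent death logic.
; On death it spawns the replacement with the BT_TDChar behavior tree at its location, passes the saved destination to the new TDAIController, then expires shortly after.
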(event `self.Die`
  (set `self.SavedDest` (`BlackboardComponent.GetValueAsVector` (`AIBlueprintHelperLibrary.GetBlackboard` (`self.GetController`)) (`KismetStringLibrary.Conv_StringToName` "Destination")))
  (`parent.Die`))

(event `self.OnDeath`
  (bind _returnvalue (`AIBlueprintHelperLibrary.SpawnAIFromClass` "/Game/Blueprint/Unit/EnemyMelee05_1.EnemyMelee05_1_C" "/Game/Blueprint/AI/BT_TDChar.BT_TDChar" (`self.K2_GetActorLocation`) (struct) true))
  (bind _astdaicontroller (cast `TDAIController` (`self.GetController` _returnvalue)))
  (`TDAIController.SetDestination` _astdaicontroller (`self.SavedDest`))
  (`self.SetLifeSpan` 0.25))

(fn `UserConstructionScript`)