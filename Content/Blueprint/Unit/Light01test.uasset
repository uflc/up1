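; Light01test is a unit Blueprint, apparently a test variant, that overrides attack and death events.
; ExecuteAttack applies the unit's attack damage to a valid AggroTarget, along with a brief shake effect.
; CharacterDestroy awards coins and calls the destroy implementation, guarded so it is skipped when the unit is already Dead.
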(event `self.ReceiveBeginPlay`)

(event `self.CharacterDestroy`
  (if (not (`|EnumEquality` (`self.UnitState`) "Dead"))
    (`MyBlueprintFunctionLibrary.EarnCoin` self 3)
    (`self.CharacterDestroy_Implementation`)))

(event `self.ExecuteAttack`
  (bind _aggrotarget (`self.AggroTarget`))
  (`/Engine/EditorBlueprintResources/StandardMacros.IsValid` _aggrotarget
    (:`Is Valid`
      (`self.ApplyDamage` _aggrotarget 12.0 0.2 (`self.UnitAttackDamage`)))))

(fn `UserConstructionScript`)