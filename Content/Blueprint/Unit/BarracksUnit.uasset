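; BarracksUnit is a unit Blueprint with a widget-based health bar that announces its own death.
; Die runs the parent logic, then fires the OnDied dispatcher with itself so listeners know which unit died.
; BeginPlay calls the parent, then prints debug positions for the actor, the HealthBar component and the bar's render translation inside its CharacterHealthBar widget.
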(event `self.Die`
  (`parent.Die`)
  (`self.OnDied` self))

(event `self.ReceiveBeginPlay`
  (bind _healthbar (`self.HealthBar`))
  (`parent.ReceiveBeginPlay`)
  (`KismetSystemLibrary.PrintString` (`KismetStringLibrary.Conv_VectorToString` (`self.K2_GetActorLocation`)))
  (`KismetSystemLibrary.PrintString` (`KismetStringLibrary.Conv_VectorToString` (`SceneComponent.K2_GetComponentLocation` _healthbar)))
  (bind _ascharacter_health_bar (cast `/Game/Blueprint/UI/CharacterHealthBar` (`WidgetComponent.GetUserWidgetObject` _healthbar)))
  (`KismetSystemLibrary.PrintString` (`KismetStringLibrary.Conv_Vector2dToString` (`.Translation` (break `WidgetTransform` (`Widget.RenderTransform` (`/Game/Blueprint/UI/CharacterHealthBar.HealthBar` _ascharacter_health_bar)))))))

(fn `UserConstructionScript`)