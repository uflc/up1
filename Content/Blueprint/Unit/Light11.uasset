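; Light11 is a tower-defense unit Blueprint that defines what happens when this enemy dies.
; On Die it switches to the Dying state, stops animation looping, unpossesses its controller and removes its health bar.
; It then awards the player coins through TDPlayerController and sets its lifespan to the death flipbook's length, replacing the parent Die logic.
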(event `self.Die`
  (`self.ChangeState` "Dying")
  (`PaperFlipbookComponent.SetLooping` (`self.Animation`) false)
  (`Controller.UnPossess` (`self.GetController`))
  (`ActorComponent.K2_DestroyComponent` (`self.HealthBar`))
  (bind _astdplayer_controller (cast `TDPlayerController` (`GameplayStatics.GetPlayerController` 0)))
  (`TDPlayerController.UpdateValue` _astdplayer_controller 3 "Coin")
  (`self.SetLifeSpan` (`PaperFlipbookComponent.GetFlipbookLength` (`self.Animation`))))

(fn `UserConstructionScript`)