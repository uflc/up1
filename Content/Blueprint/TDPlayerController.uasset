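; Player controller for the tower defense game that manages the camera and touch input.
; On level change it spawns a top-down orthographic camera if needed, then sets ortho width and pan limit from map size.
; Touch either hides the tower menu or starts clamped horizontal panning, which shifts the HUD's tower widget to follow.
; A test event sets barracks rally points within an X-scaled, elliptical tower range.
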(event `Testing_pc`
  (bind (_locationx _locationy) (`self.GetMousePosition`))
  (bind _worldposition (`GameplayStatics.DeprojectScreenToWorld` self (`KismetMathLibrary.MakeVector2D` _locationx _locationy)))
  (if (`self.IsWaitingForNextTouch`)
    (bind _astdgame_mode_base (cast `TDGameModeBase` (`GameplayStatics.GetGameMode`)))
    (bind _returnvalue (`TDGameModeBase.GetCurrentWidget` _astdgame_mode_base))
    (`/Engine/EditorBlueprintResources/StandardMacros.IsValid` _returnvalue
      (:`Is Valid`
        (bind _ashud (cast `/Game/Blueprint/UI/HUD` _returnvalue))
        (bind _owntower (`UITowerBase.OwnTower` (`/Game/Blueprint/UI/HUD.vUITower` _ashud)))
        (if (> (`KismetMathLibrary.VSize` (* (- _worldposition (`self.K2_GetActorLocation` _owntower)) (0.666667 1.0 1.0))) (`Tower.GetTowerRange` _owntower))
          (`KismetSystemLibrary.PrintString` "Out Of Range")
          (else
            (bind _asbptower_barracks (cast `/Game/Blueprint/Tower/Building/BPTowerBarracks` _owntower))
            (`/Game/Blueprint/Tower/Building/BPTowerBarracks.Set Rally Point` _asbptower_barracks _worldposition)
            (`KismetSystemLibrary.PrintString` "In Range")))))))

(event `LevelChange`
  (params (`Map Size` :type "Vector2D Structure"))
  (`/Engine/EditorBlueprintResources/StandardMacros.IsValid` (`self.ViewCameraActor`)
    (:`Is Valid`
      _)
    (:`Is Not Valid`
      (bind _returnvalue (`|SpawnActorFromClass` "/Script/Engine.CameraActor" (`KismetMathLibrary.MakeTransform` (0.0 0.0 500.0) (struct :`Pitch` -90.0 :`Roll` -90.0)) "Undefined" "OverrideRootScale" null null))
      (bind _output_get (set `self.ViewCameraActor` _returnvalue))
      (`self.SetViewTargetWithBlend` _output_get)
      (bind _cameracomponent (`CameraActor.CameraComponent` _returnvalue))
      (`CameraComponent.SetProjectionMode` _cameracomponent "Orthographic")
      (`CameraComponent.SetConstraintAspectRatio` _cameracomponent false)))
  (`self.SetCameraFitToMap` `Map Size`))

(event `InputAction|PlayerTouched`
  (params (Key :type "Key Structure"))
  (:`Pressed`
    (if (`self.IsWaitingForNextTouch`)
      (set `self.IsWaitingForNextTouch` false)
      (bind _astdgame_mode_base (cast `TDGameModeBase` (`GameplayStatics.GetGameMode`)))
      (bind _returnvalue (`TDGameModeBase.GetCurrentWidget` _astdgame_mode_base))
      (`/Engine/EditorBlueprintResources/StandardMacros.IsValid` _returnvalue
        (:`Is Valid`
          (bind _ashud (cast `/Game/Blueprint/UI/HUD` _returnvalue))
          (`HUDWidget.HideTowerActionMenu` _ashud)))
      (else
        (`/Engine/EditorBlueprintResources/StandardMacros.IsValid` (`self.ViewCameraActor`)
          (:`Is Valid`
            (set `self.IsCameraPanning` true))))))
  (:`Released`
    (set `self.IsCameraPanning` false)))

(event `InputAxis|ScreenScrollX`
  (params (AxisValue :type "Float (single-precision)"))
  (bind _returnvalue (* AxisValue (`self.CameraSpeed`)))
  (bind _returnvalue_x (`KismetMathLibrary.BreakVector` (`SceneComponent.K2_GetComponentLocation` (`Actor.RootComponent` (`self.ViewCameraActor`)))))
  ;[1 1 1] 카메라 패닝
  (if (`self.IsCameraPanning`)
    (if (< (`KismetMathLibrary.Abs` (+ _returnvalue _returnvalue_x)) (`self.PanThreshold`))
      (`SceneComponent.K2_AddWorldOffset` (`Actor.RootComponent` (`self.ViewCameraActor`)) (`KismetMathLibrary.MakeVector` _returnvalue) false false)
      (bind _astdgame_mode_base (cast `TDGameModeBase` (`GameplayStatics.GetGameMode`)))
      (bind _returnvalue_2 (`TDGameModeBase.GetCurrentWidget` _astdgame_mode_base))
      (`/Engine/EditorBlueprintResources/StandardMacros.IsValid` _returnvalue_2
        (:`Is Valid`
          (bind _ashud (cast `/Game/Blueprint/UI/HUD` _returnvalue_2))
          (bind _returnvalue_3 (`WidgetLayoutLibrary.SlotAsCanvasSlot` (`/Game/Blueprint/UI/HUD.vUITower` _ashud)))
          (`CanvasPanelSlot.SetPosition` _returnvalue_3 (- (`CanvasPanelSlot.GetPosition` _returnvalue_3) (`KismetMathLibrary.MakeVector2D` (* _returnvalue 0.582)))))))))

(fn `SetCameraFitToMap`
  (params (`Map Size` :type "Vector2D Structure"))
  (bind (_x _y) (`KismetMathLibrary.BreakVector2D` `Map Size`))
  (bind _returnvalue (* (`CameraComponent.AspectRatio` (`CameraActor.CameraComponent` (`self.ViewCameraActor`))) _y))
  (set `self.PanThreshold` (/ (- _x _returnvalue) 2.0))
  (`CameraComponent.SetOrthoWidth` (`CameraActor.CameraComponent` (`self.ViewCameraActor`)) _returnvalue))

(fn `UserConstructionScript`)