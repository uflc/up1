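; Test tower spawner actor that fills a square grid with empty tower actors when play begins.
; BeginPlay runs a single loop over Size squared cells, using modulo and division by Size to turn each index into a column and row.
; Each cell is scaled by BlockSpacing, offset from the spawner's location at a slight fixed height, and gets a BPTowerEmpty spawned regardless of collision.
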(event `self.ReceiveBeginPlay`
  (bind _size (`self.Size`))
  (bind _size_2 (`self.Size`))
  (bind _blockspacing (`self.BlockSpacing`))
  ;[1 1 1] Spawn Test Towers
  (for _index (range (* _size _size))
    (`|SpawnActorFromClass` "/Game/Blueprint/Tower/BPTowerEmpty.BPTowerEmpty_C" (`KismetMathLibrary.Conv_VectorToTransform` (+ (`KismetMathLibrary.MakeVector` (* (mod _index _size_2) _blockspacing) (* (/ _index _size_2) _blockspacing) 10.0) (`self.K2_GetActorLocation`))) "AlwaysSpawn" "OverrideRootScale" null null) ; Spawn a  block
  ))

(fn `UserConstructionScript`)