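; TDPlayerState is the player state that holds the player's Coin, Life, Mana and Hero HP values.
; UpdateValue overwrites the variable selected by the Type argument with the given value.
; It then fetches the current widget from MyUMGGameModeBase and, if that is a valid HUD, forwards the value and type to its UpdateValues.
; BeginPlay, Tick and the construction script are empty.
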(fn `UpdateValue`
  (params (Value :type Integer) (Type :type "/Game/Blueprint/UI/ValueType Enum" :default "NewEnumerator0"))
  (switch `/Game/Blueprint/UI/ValueType` Type
    (:`NewEnumerator0`
      (set `self.Coin` Value))
    (:`NewEnumerator1`
      (set `self.Life` Value))
    (:`NewEnumerator2`
      (set `self.Mana` Value))
    (:`NewEnumerator3`
      (set `self.HeroHP` Value)))
  (bind _asmy_umggame_mode_base (cast `MyUMGGameModeBase` (`GameplayStatics.GetGameMode`)))
  (bind _returnvalue (`MyUMGGameModeBase.GetCurrentWidget` _asmy_umggame_mode_base))
  (`/Engine/EditorBlueprintResources/StandardMacros.IsValid` _returnvalue
    (:`Is Valid`
      (bind _ashud (cast `/Game/Blueprint/UI/HUD` _returnvalue))
      (`/Game/Blueprint/UI/HUD.UpdateValues` _ashud Value Type))))

(fn `UserConstructionScript`)