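; Behavior Tree decorator that tests whether the AI-controlled pawn is actually moving.
; It passes when absolute velocity exceeds a small threshold on both X and Y.
; Otherwise it alternates between storing the location and passing, then comparing displacement from that stored point on the next check.
; An older timer-based velocity check remains disconnected, with a debug print in its event.
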(event `VelocityCheck`
  (set `self.bIsPendingVelocityCheck` false)
  (set `self.bIsActuallyMoving` false)
  (`KismetSystemLibrary.PrintString` "Hello")
  (`KismetSystemLibrary.K2_ClearAndInvalidateTimerHandle` (`self.VelocityCheckTimer`)))

(fn `PerformConditionCheckAI`
  (params (OwnerController :type "AIController Object Reference") (ControlledPawn :type "Pawn Object Reference"))
  (returns (ReturnValue :type Boolean))
  (locals (bRetVal :type Boolean))
  (bind (_returnvalue_x _returnvalue_y) (`KismetMathLibrary.BreakVector` (`KismetMathLibrary.Vector_GetAbs` (`MovementComponent.Velocity` (`Pawn.GetMovementComponent` ControlledPawn)))))
  (bind (_returnvalue_x_2 _returnvalue_y_2) (`KismetMathLibrary.BreakVector` (`KismetMathLibrary.Vector_GetAbs` (- (`self.StoppedPoint`) (`Actor.K2_GetActorLocation` (`self.Pawn`))))))
  (`/Engine/EditorBlueprintResources/StandardMacros.IsValid` ControlledPawn
    (:`Is Valid`
      (if (and (> _returnvalue_x 1.0) (> _returnvalue_y 1.0))
        (return true)
        (elif (`self.bNeedLocationCheck`)
          (set `self.bNeedLocationCheck` false)
          (return (and (> _returnvalue_x_2 1.0) (> _returnvalue_y_2 1.0)))
          (else
            (set `self.StoppedPoint` (`Actor.K2_GetActorLocation` (`self.Pawn`)))
            (set `self.bNeedLocationCheck` true)
            (return true)))))))