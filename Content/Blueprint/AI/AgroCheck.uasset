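; AI Behavior Tree tick logic that picks an aggro target for an enemy Paper character and writes its location to the TargetLocation blackboard key.
; Each tick it caches the AI controller and sphere-traces around the pawn at its AggroDrawnRange, ignoring same-team characters.
; Hits passing a DrawingAggroRange threshold compete by distance, though the comparison replaces the stored target with farther hits despite the ClosestDistance name.
; The trace leaves persistent debug drawing.
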(event `self.ReceiveTick`
  (params (OwnerActor :type "Actor Object Reference") (DeltaSeconds :type "Float (single-precision)"))
  (bind _aggrotarget (`self.AggroTarget`))
  (bind _returnvalue (`Controller.K2_GetPawn` (`self.AI CON Ref`)))
  ;[1 1 1] Is AI CON set?
  (if (not (!= (`self.AI CON Ref`) null))
    (bind _asai_enemy_controller (cast `/Game/Blueprint/AI/AI_EnemyController` OwnerActor))
    (set `self.AI CON Ref` _asai_enemy_controller))
  (bind _outactors (`GameplayStatics.GetAllActorsOfClass` "/Script/work2.MyPaperCharacter"))
  ;[1 1 1] Make array of team units to be ignored on tracing for Aggro check
  (set `self.TeamUnits` _outactors)
  (for _array_element _outactors
    (if (`|EnumInequality` (`MyPaperCharacter.Team` _array_element) (`MyPaperCharacter.Team` (stale _asmy_paper_character)))
      (`KismetArrayLibrary.Array_RemoveItem` (`self.TeamUnits`) _array_element)))
  (bind _asmy_paper_character (cast `MyPaperCharacter` _returnvalue))
  (bind _output_get (set `self.MyLocation` (`Actor.K2_GetActorLocation` _returnvalue)))
  (bind _outhits (`KismetSystemLibrary.SphereTraceMultiForObjects` _output_get _output_get (`MyPaperCharacter.AggroDrawnRange` _asmy_paper_character) (`self.DesiredObjectTypes`) false (`self.TeamUnits`) "Persistent"))
  (for _array_element_2 _outhits
    (bind (_bblockinghit _binitialoverlap _time _distance _location _impactpoint _normal _impactnormal _physmat _hitactor) (`GameplayStatics.BreakHitResult` _array_element_2))
    (bind _asmy_paper_character_2 (cast `MyPaperCharacter` _hitactor))
    (if (>= (`MyPaperCharacter.DrawingAggroRange` _asmy_paper_character_2) 0.0)
      (`/Engine/EditorBlueprintResources/StandardMacros.IsValid` (`self.AggroTarget`)
        (:`Is Valid`
          (if (< (`self.ClosestDistance`) _distance)
            (set `self.ClosestDistance` _distance)
            (set `self.AggroTarget` _asmy_paper_character_2)))
        (:`Is Not Valid`
          (set `self.AggroTarget` _asmy_paper_character_2)
          (set `self.ClosestDistance` _distance)))))
  (`/Engine/EditorBlueprintResources/StandardMacros.IsValid` _aggrotarget
    (:`Is Valid`
      (`BTFunctionLibrary.SetBlackboardValueAsVector` (`self.TargetLocation`) (`Actor.K2_GetActorLocation` _aggrotarget)))))