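; Behavior tree AI check that looks for an aggro target around the enemy controller's pawn on each tick.
; It caches the AI controller, then sphere-traces by the pawn's AggroDrawnRange for paper characters whose DrawingAggroRange covers the hit distance.
; The comparison favors farther hits despite the ClosestDistance name, and a valid AggroTarget triggers a write to AggroTargetKey.
; Team-filtering logic for trace ignores is present but unconnected.
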(event `self.ReceiveTick`
  (params (OwnerActor :type "Actor Object Reference") (DeltaSeconds :type "Float (single-precision)"))
  (bind _returnvalue (`Controller.K2_GetPawn` (`self.AI CON Ref`)))
  ;[1 1 1] Is AI CON set?
  (if (not (!= (`self.AI CON Ref`) null))
    (bind _asai_enemy_controller (cast `/Game/Blueprint/AI/AI_EnemyController` OwnerActor))
    (set `self.AI CON Ref` _asai_enemy_controller))
  (bind _outactors (`GameplayStatics.GetAllActorsOfClass` "/Script/work2.MyPaperCharacter"))
  (bind _asmy_paper_character (cast `MyPaperCharacter` _returnvalue))
  (bind _output_get (set `self.MyLocation` (`Actor.K2_GetActorLocation` _returnvalue)))
  (bind _outhits (`KismetSystemLibrary.SphereTraceMultiForObjects` _output_get (+ _output_get (0.0 0.0 1.0)) (`MyPaperCharacter.AggroDrawnRange` _asmy_paper_character) (`self.DesiredObjectTypes`)))
  (for (_array_element _array_index) _outhits
    (`KismetSystemLibrary.PrintString` (`KismetStringLibrary.Conv_IntToString` _array_index))
    (bind (_bblockinghit _binitialoverlap _time _distance _location _impactpoint _normal _impactnormal _physmat _hitactor) (`GameplayStatics.BreakHitResult` _array_element))
    (bind _asmy_paper_character_2 (cast `MyPaperCharacter` _hitactor))
    (if (>= (`MyPaperCharacter.DrawingAggroRange` _asmy_paper_character_2) _distance)
      (`/Engine/EditorBlueprintResources/StandardMacros.IsValid` (`self.AggroTarget`)
        (:`Is Valid`
          (if (< (`self.ClosestDistance`) _distance)
            (set `self.ClosestDistance` _distance)
            (set `self.AggroTarget` _asmy_paper_character_2)))
        (:`Is Not Valid`
          (set `self.AggroTarget` _asmy_paper_character_2)
          (set `self.ClosestDistance` _distance)))))
  (`/Engine/EditorBlueprintResources/StandardMacros.IsValid` (`self.AggroTarget`)
    (:`Is Valid`
      (`BTFunctionLibrary.SetBlackboardValueAsObject` (`self.AggroTargetKey`)))))