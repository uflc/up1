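; Behavior tree service that picks the nearest aggro target for an AI-controlled enemy TDUnit.
; Each tick it sphere-traces at the pawn within AggroDrawnRange, ignoring units of its own team or with no team.
; It keeps the closest hit whose own DrawingAggroRange covers the planar distance.
; It writes that target and an in-attack-range flag to the Blackboard, clearing the target when the trace finds nothing.
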(event `self.ReceiveTick`
  (params (OwnerActor :type "Actor Object Reference") (DeltaSeconds :type "Float (single-precision)"))
  (bind _aggrotargetkey (`self.AggroTargetKey`))
  (bind _aggrotarget (`self.AggroTarget`))
  (bind _aggrotarget_2 (`self.AggroTarget`))
  (bind _returnvalue (`Controller.K2_GetPawn` (`self.AI CON Ref`)))
  ;[1 1 1] Is AI CON set?
  (if (not (!= (`self.AI CON Ref`) null))
    (bind _asai_enemy_unit_controller (cast `/Game/Blueprint/AI/AI_EnemyUnitController` OwnerActor))
    (set `self.AI CON Ref` _asai_enemy_unit_controller))
  ;[1 1 1] Update current DistanceToTarget value, if Aggro Target was set
  (`/Engine/EditorBlueprintResources/StandardMacros.IsValid` _aggrotarget
    (:`Is Valid`
      (set `self.DistanceToTarget` (`KismetMathLibrary.VSizeXY` (- (`Actor.K2_GetActorLocation` _aggrotarget) (`self.MyLocation`)))))
    (:`Is Not Valid`
      _))
  (bind _outactors (`GameplayStatics.GetAllActorsOfClass` "/Script/TowerDefense.TDUnit"))
  (bind _astdunit (cast `TDUnit` _returnvalue))
  (bind _output_get (set `self.MyLocation` (`Actor.K2_GetActorLocation` _returnvalue)))
  ;[1 1 1] Make array of team units to be ignored on tracing
  (for _array_element _outactors
    (bind _team (`TDUnit.Team` _array_element))
    (if (or (`|EnumEquality` _team) (`|EnumEquality` _team (`TDUnit.Team` _astdunit)))
      (`KismetArrayLibrary.Array_AddUnique` (`self.TeamUnits`) _array_element)))
  (bind (_outhits _returnvalue_2) (`KismetSystemLibrary.SphereTraceMultiForObjects` _output_get (+ _output_get (0.0 0.0 0.1)) (`TDUnit.AggroDrawnRange` _astdunit) (`self.DesiredObjectTypes`) false (`self.TeamUnits`)))
  (for _array_element_2 _outhits
    (bind (_bblockinghit _binitialoverlap _time _distance _location _impactpoint _normal _impactnormal _physmat _hitactor _hitcomponent _hitbonename _hititem _faceindex _tracestart) (`GameplayStatics.BreakHitResult` _array_element_2))
    (bind _astdunit_2 (cast `TDUnit` _hitactor))
    (bind _returnvalue_3 (`KismetMathLibrary.VSizeXY` (- (`Actor.K2_GetActorLocation` _hitactor) _tracestart)))
    (if (>= (`TDUnit.DrawingAggroRange` _astdunit_2) _returnvalue_3)
      (`/Engine/EditorBlueprintResources/StandardMacros.IsValid` (`self.AggroTarget`)
        (:`Is Valid`
          (if (> (`self.DistanceToTarget`) _returnvalue_3)
            (set `self.DistanceToTarget` _returnvalue_3)
            (set `self.AggroTarget` _astdunit_2)))
        (:`Is Not Valid`
          (set `self.AggroTarget` _astdunit_2)
          (set `self.DistanceToTarget` _returnvalue_3)))))
  (if _returnvalue_2
    (`/Engine/EditorBlueprintResources/StandardMacros.IsValid` _aggrotarget_2
      (:`Is Valid`
        (`BTFunctionLibrary.SetBlackboardValueAsObject` _aggrotargetkey _aggrotarget_2)
        (`BlackboardComponent.SetValueAsBool` (`BTFunctionLibrary.GetOwnersBlackboard`) (`self.CanAttackTargetKey`) (>= (`TDUnit.AttackRange` _astdunit) (`self.DistanceToTarget`)))))
    (else
      (`/Engine/EditorBlueprintResources/StandardMacros.IsValid` _aggrotarget_2
        (:`Is Valid`
          (set `self.AggroTarget` null)
          (`BTFunctionLibrary.SetBlackboardValueAsObject` _aggrotargetkey))))))