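; Behavior tree task that makes an AI-controlled TDUnit attack the aggro target stored in the blackboard.
; It sets the delay-checker key to true, calls ExecAttack on the pawn's AttackComponent, and has the AI controller start a timer on that key using the unit's attack delay.
; The task finishes successfully after a timer as long as the sprite's current flipbook, separating animation length from attack cooldown.
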(event `self.ReceiveExecute`
  (params (OwnerActor :type "Actor Object Reference"))
  (bind _returnvalue (`AIBlueprintHelperLibrary.GetAIController` OwnerActor))
  (bind _delaycheckerkey (`self.DelayCheckerKey`))
  (bind _returnvalue_2 (`Controller.K2_GetPawn` _returnvalue))
  (bind _asai_unit_controller_base (cast `/Game/Blueprint/AI/AI_UnitControllerBase` _returnvalue))
  (bind _astdunit (cast `TDUnit` _returnvalue_2))
  (`BTFunctionLibrary.SetBlackboardValueAsBool` _delaycheckerkey true)
  (`AttackComponent.ExecAttack` (`Actor.GetComponentByClass` _returnvalue_2 "/Script/TowerDefense.AttackComponent") (`BTFunctionLibrary.GetBlackboardValueAsObject` (`self.AggroTargetKey`)))
  (`/Game/Blueprint/AI/AI_UnitControllerBase.Set TImer of AI Con` _asai_unit_controller_base (`TDUnit.UnitAttackDelay` _astdunit) (`.SelectedKeyName` (break `BlackboardKeySelector` _delaycheckerkey)))
  (`KismetSystemLibrary.K2_SetTimerDelegate` (delegate `TimerEnd`) (`PaperFlipbook.GetTotalDuration` (`PaperFlipbookComponent.GetFlipbook` (`PaperCharacter.Sprite` _astdunit)))))

(event `TimerEnd`
  (`self.FinishExecute` true))