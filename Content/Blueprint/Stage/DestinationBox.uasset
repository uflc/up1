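; DestinationBox is a tower-defense waypoint that routes overlapping enemy characters toward their next destination.
; On overlap it sends the enemy's AI controller to a box in its Next list, or calls Finish on the enemy when that list is empty.
; At forks, it pops the branch index from the front of the AI controller's DestBranchIdxQ queue, defaulting to the first entry when the queue is empty.
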(event `self.ReceiveActorBeginOverlap`
  (params (OtherActor :type "Actor Object Reference"))
  (bind _asenemy_tdcharacter (cast `EnemyTDCharacter` OtherActor))
  (if (`KismetArrayLibrary.Array_IsValidIndex` (`self.Next`))
    (bind _asenemy_tdchar_aicontroller (cast `EnemyTDCharAIController` (`AIBlueprintHelperLibrary.GetAIController` _asenemy_tdcharacter)))
    (if (not (== (`KismetArrayLibrary.Array_Length` (`self.Next`)) 1))
      (bind _destination_index (`self.Get Enemy Destination Index` _asenemy_tdchar_aicontroller)))
    (`self.Set Enemy Destination` _destination_index _asenemy_tdchar_aicontroller)
    (else
      (`EnemyTDCharacter.Finish` _asenemy_tdcharacter))))

(fn `Get Enemy Destination Index`
  (params (`Enemy AI` :type "EnemyTDCharAIController Object Reference"))
  (returns (`Destination Index` :type Integer))
  (locals (DestinationIndex :type Integer :default 0))
  (bind _destbranchidxq (`EnemyTDCharAIController.DestBranchIdxQ` `Enemy AI`))
  (if (`KismetArrayLibrary.Array_IsValidIndex` _destbranchidxq)
    (set `local.DestinationIndex` (`KismetMathLibrary.Conv_ByteToInt` (`|GetArrayItem` _destbranchidxq)))
    (`KismetArrayLibrary.Array_Remove` _destbranchidxq)
    (return (`local.DestinationIndex`))
    (else
      (return 0))))

(fn `Set Enemy Destination`
  (params (`Destinaion Index` :type Integer) (EnemyAI :type "TDCharAIController Object Reference"))
  (bind _output (`|GetArrayItem` (`self.Next`) `Destinaion Index`))
  (`/Engine/EditorBlueprintResources/StandardMacros.IsValid` _output
    (:`Is Valid`
      (`TDCharAIController.SetDestination` EnemyAI (`self.K2_GetActorLocation` _output)))
    (:`Is Not Valid`
      (`KismetSystemLibrary.PrintString` "Next Destination is NOT set"))))

(fn `UserConstructionScript`)