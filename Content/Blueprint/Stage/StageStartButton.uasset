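; Stage start button sprite that continuously pulses its opacity; it contains no click or stage-start logic.
; Tick moves an Alpha accumulator up or down by delta time, flipping the IsIncreasing flag at the bounds for a ping-pong fade of about two seconds each way.
; The halved value sets the white sprite color's alpha on the render component.
; A leftover debug print fires every frame.
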(event `self.ReceiveBeginPlay`
  (`self.SetActorTickEnabled` true))

(event `self.ReceiveTick`
  (params (DeltaSeconds :type "Float (single-precision)"))
  (if (`self.IsIncreasing`)
    (set `self.Alpha` (+ DeltaSeconds (`self.Alpha`)))
    (else
      (set `self.Alpha` (- (`self.Alpha`) DeltaSeconds))))
  (`PaperFlipbookComponent.SetSpriteColor` (`self.RenderComponent`) (make `LinearColor` 1.0 1.0 1.0 (/ (`self.Alpha`) 2.0)))
  (`KismetSystemLibrary.PrintString` "Hello")
  (if (`self.IsIncreasing`)
    (if (>= (`self.Alpha`) 2.0)
      (set `self.IsIncreasing` false))
    (elif (>= 0.0 (`self.Alpha`))
      (set `self.IsIncreasing` true))))

(fn `UserConstructionScript`)