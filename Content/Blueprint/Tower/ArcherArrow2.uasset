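; ArcherArrow2 is an arrow projectile actor that homes in on a Target at a set Velocity.
; Each Tick it teleports along the flattened XY direction to the target, facing that yaw plus 180 degrees.
; A zero result from the tolerance-based normalize serves as the hit test, triggering ApplyDamage with shake parameters but zero damage, then destruction.
; An invalid target jumps to that same damage-and-destroy path.
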(event `self.ReceiveTick`
  (params (DeltaSeconds :type "Float (single-precision)"))
  (bind _returnvalue (`self.K2_GetActorLocation`))
  (bind _target (`self.Target`))
  (bind _returnvalue_2 (`KismetMathLibrary.Vector_Normal2D` (`KismetMathLibrary.Conv_Vector2DToVector` (`KismetMathLibrary.Conv_VectorToVector2D` (- (`self.K2_GetActorLocation` _target) _returnvalue))) 100.0))
  (`/Engine/EditorBlueprintResources/StandardMacros.IsValid` _target
    (:`Is Valid`
      (if (`KismetMathLibrary.Vector_IsZero` _returnvalue_2)
        (`MyPaperCharacter.ApplyDamage` (`self.Target`) 8.0 0.15 0 :!label _label)
        (`self.K2_DestroyActor`)
        (else
          (`self.K2_TeleportTo` (+ (* (* _returnvalue_2 (`self.Velocity`)) DeltaSeconds) _returnvalue) (`KismetMathLibrary.MakeRotator` 0.0 0.0 (+ (`KismetMathLibrary.GetYawPitchFromVector` _returnvalue_2) 180.0))))))
    (:`Is Not Valid`
      (goto _label))))

(fn `UserConstructionScript`)